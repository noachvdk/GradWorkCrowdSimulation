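; Crowd pedestrian character that registers itself with the CPP_CrowdManager on BeginPlay and can switch between a default mesh and a randomized modular appearance.
; UpdateVisualTraits passes gender to the pedestrian controller's navigation filter, then picks random gendered body, head, hands, legs and hair meshes.
; DefaultVisualTraits restores the placeholder mesh.
; Construction slaves body parts to the main mesh via master pose and snaps hair and eyes to the head socket.
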(event `self.ReceiveBeginPlay`
  (`parent.ReceiveBeginPlay`)
  (bind _returnvalue (`GameplayStatics.GetActorOfClass` "/Script/CrowdSimulationV4.CPP_CrowdManager"))
  (`/Engine/EditorBlueprintResources/StandardMacros.IsValid` _returnvalue
    (:`Is Valid`
      (`CPP_CrowdManager.AddPedestrian` _returnvalue self))))

(event `self.UpdateVisualTraits`
  (bind _maleheadmeshes (`self.MaleHeadMeshes`))
  (bind _femaleheadmeshes (`self.FemaleHeadMeshes`))
  (bind _ismale (`self.IsMale`))
  (bind _malehandmeshes (`self.MaleHandMeshes`))
  (bind _femalehandmeshes (`self.FemaleHandMeshes`))
  (bind _malelegmeshes (`self.MaleLegMeshes`))
  (bind _femalelegmeshes (`self.FemaleLegMeshes`))
  (bind _malehairmeshes (`self.MaleHairMeshes`))
  (bind _femalehairmeshes (`self.FemaleHairMeshes`))
  (bind _malebodymeshes (`self.MaleBodyMeshes`))
  (bind _femalebodymeshes (`self.FemaleBodyMeshes`))
  ;[1 1 1] Update navigation query filter
  (bind _asbp_pedestrian_controller (cast `/Game/Crowd/BP_PedestrianController` (`self.GetController`))
    (:`then`
      (`/Game/Crowd/BP_PedestrianController.SetNavigationFilter` _asbp_pedestrian_controller _ismale))
    (:`CastFailed`
      _))
  ;[1 1 1] Toggle meshes
  (`SceneComponent.SetHiddenInGame` (`self.Mesh`) false true)
  (`SceneComponent.SetHiddenInGame` (`self.Default mesh`) true false)
  ;[1 1 1] Switch Model depending on gender
  (if _ismale
    ;[1 1 1] Switch body
    (`SkinnedMeshComponent.SetSkinnedAssetAndUpdate` (`self.Mesh`) (`|GetArrayItem` _malebodymeshes (`KismetMathLibrary.RandomInteger` (`KismetArrayLibrary.Array_Length` _malebodymeshes))) true)
    ;[1 1 1] Switch head
    (`SkinnedMeshComponent.SetSkinnedAssetAndUpdate` (`self.Head`) (`|GetArrayItem` _maleheadmeshes (`KismetMathLibrary.RandomInteger` (`KismetArrayLibrary.Array_Length` _maleheadmeshes))) true)
    ;[1 1 1] Switch hands
    (`SkinnedMeshComponent.SetSkinnedAssetAndUpdate` (`self.Hands`) (`|GetArrayItem` _malehandmeshes (`KismetMathLibrary.RandomInteger` (`KismetArrayLibrary.Array_Length` _malehandmeshes))) true)
    ;[1 1 1] Switch legs
    (`SkinnedMeshComponent.SetSkinnedAssetAndUpdate` (`self.Legs`) (`|GetArrayItem` _malelegmeshes (`KismetMathLibrary.RandomInteger` (`KismetArrayLibrary.Array_Length` _malelegmeshes))) true)
    ;[1 1 1] Switch hair
    (`StaticMeshComponent.SetStaticMesh` (`self.Hair`) (`|GetArrayItem` _malehairmeshes (`KismetMathLibrary.RandomInteger` (`KismetArrayLibrary.Array_Length` _malehairmeshes))))
    (else
      (`SkinnedMeshComponent.SetSkinnedAssetAndUpdate` (`self.Mesh`) (`|GetArrayItem` _femalebodymeshes (`KismetMathLibrary.RandomInteger` (`KismetArrayLibrary.Array_Length` _femalebodymeshes))) true)
      (`SkinnedMeshComponent.SetSkinnedAssetAndUpdate` (`self.Head`) (`|GetArrayItem` _femaleheadmeshes (`KismetMathLibrary.RandomInteger` (`KismetArrayLibrary.Array_Length` _femaleheadmeshes))) true)
      (`SkinnedMeshComponent.SetSkinnedAssetAndUpdate` (`self.Hands`) (`|GetArrayItem` _femalehandmeshes (`KismetMathLibrary.RandomInteger` (`KismetArrayLibrary.Array_Length` _femalehandmeshes))) true)
      (`SkinnedMeshComponent.SetSkinnedAssetAndUpdate` (`self.Legs`) (`|GetArrayItem` _femalelegmeshes (`KismetMathLibrary.RandomInteger` (`KismetArrayLibrary.Array_Length` _femalelegmeshes))) true)
      (`StaticMeshComponent.SetStaticMesh` (`self.Hair`) (`|GetArrayItem` _femalehairmeshes (`KismetMathLibrary.RandomInteger` (`KismetArrayLibrary.Array_Length` _femalehairmeshes)))))))

(event `self.DefaultVisualTraits`
  ;[1 1 1] Reset to default mesh
  (`SceneComponent.SetHiddenInGame` (`self.Mesh`) true true)
  (`SceneComponent.SetHiddenInGame` (`self.Default mesh`) false false))

(fn `UserConstructionScript`
  (bind _mesh (`self.Mesh`))
  (`SkinnedMeshComponent.SetLeaderPoseComponent` (`self.Hands`) _mesh false)
  (`SkinnedMeshComponent.SetLeaderPoseComponent` (`self.Head`) _mesh false)
  (`SkinnedMeshComponent.SetLeaderPoseComponent` (`self.Legs`) _mesh false)
  (`SceneComponent.K2_AttachToComponent` (`self.Hair`) _mesh "headSocket" "SnapToTarget" "SnapToTarget" "KeepRelative" true)
  (`SceneComponent.K2_AttachToComponent` (`self.Eyes`) _mesh "headSocket" "SnapToTarget" "SnapToTarget" "KeepRelative" true))