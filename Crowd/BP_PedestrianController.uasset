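; Controller for crowd pedestrians that picks each next walk destination and sets a male or female navigation filter, caching the CPP_CrowdManager on BeginPlay.
; CalcNextPoint runs bounded, growing sphere traces ahead of the pawn on a custom object channel, choosing a random path point other than the previous one.
; It passes a random navigable location near that point to SetTargetAndDirection.
; Failed searches turn the pawn slightly and retry after a delay.
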(event `SetNavigationFilter`
  (params (IsMale :type Boolean))
  ;[1 1 1] Set Navigation filter
  (if IsMale
    (set `self.DefaultNavigationFilterClass` "/Game/Pathing/Nav/BP_QueryFilter_Male.BP_QueryFilter_Male_C")
    (else
      (set `self.DefaultNavigationFilterClass` "/Game/Pathing/Nav/BP_QueryFilter_FeMale.BP_QueryFilter_Female_C"))))

(event `self.ReceiveBeginPlay`
  ;[1 1 1] set crowd manager
  (`parent.ReceiveBeginPlay`)
  (bind _returnvalue (`GameplayStatics.GetActorOfClass` "/Script/CrowdSimulationV4.CPP_CrowdManager"))
  (`/Engine/EditorBlueprintResources/StandardMacros.IsValid` _returnvalue
    (:`Is Valid`
      (set `self.CrowdManager` _returnvalue))))

(event `self.CalcNextPoint`
  (bind _returnvalue (`self.K2_GetPawn`))
  (bind _returnvalue_2 (+ (`self.K2_GetActorLocation` _returnvalue) (* (`self.GetActorForwardVector` _returnvalue) (`self.DistanceToCheck`))))
  (set `self.IsMoving` false)
  ;[1 0.09369 0.1036] Find the next path point using a for loop to avoid infinte loop errors (Done in blueprints to be able to use the custom object channel more easily).
  (for _index (range 1 11)
    (bind _output_get (set `self.CurrentRadius` (* _index (`self.BaseCheckRadius`))))
    (bind (_outhits _returnvalue_3) (`KismetSystemLibrary.SphereTraceMultiForObjects` _returnvalue_2 (+ _returnvalue_2 (1.0 0.0 0.0)) _output_get (`|MakeArray` "ObjectTypeQuery7" :!type "EObjectTypeQuery Enum") false (`|MakeArray` (`self.PathPoint`))))
    (bind _output_get_2 (set `self.SphereCastCheck` _returnvalue_3))
    (if _output_get_2
      (set `self.PathPoint` (`.HitActor` (`GameplayStatics.BreakHitResult` (`|GetArrayItem` _outhits (`KismetMathLibrary.RandomInteger` (`KismetArrayLibrary.Array_Length` _outhits))))))
      (break)))
  ;[1 0.6012 0] If path point found go next otherwise rotate the controller a bit then retry.
  (if (`self.SphereCastCheck`)
    ;[0.8412 1 0.4214] Make sure that the path point is a reachable point
    (bind _pathpoint (`self.PathPoint`)
      (:`then`
        (for _index_2 (range 1 11)
          (bind _output_get_3 (set `self.CurrentNavCheckRadius` (* _index_2 (`self.BaseNavCheckRadius`))))
          (bind (_randomlocation _returnvalue_4) (`NavigationSystemV1.K2_GetRandomLocationInNavigableRadius` (`self.K2_GetActorLocation` _pathpoint) _output_get_3 null null))
          (bind _output_get_4 (set `self.RandomReachablePointCheck` _returnvalue_4))
          (if _output_get_4
            (set `self.RandomReachablePoint` _randomlocation)
            (break)))
        ;[1 0.6012 0] If reachable point found go next otherwise rotate the controller a bit then retry.
        (if (`self.RandomReachablePointCheck`)
          (set `self.IsMoving` true)
          (`self.SetTargetAndDirection` (`self.RandomReachablePoint`))
          (else
            (`self.K2_AddActorLocalRotation` (`self.K2_GetPawn`) (struct :`Yaw` 15.0) false false)
            (`KismetSystemLibrary.Delay` 1.0)
            (`self.CalcNextPoint`))))
      (:`else`))
    (else
      (`self.K2_AddActorLocalRotation` (`self.K2_GetPawn`) (struct :`Yaw` 15.0) false false)
      (`KismetSystemLibrary.Delay` 1.0)
      (`self.CalcNextPoint`))))

(fn `UserConstructionScript`)